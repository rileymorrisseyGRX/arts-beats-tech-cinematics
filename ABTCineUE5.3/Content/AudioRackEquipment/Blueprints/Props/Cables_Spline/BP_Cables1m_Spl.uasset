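; BP_Cables1m_Spl is an audio rack cable prop that follows an editable spline.
; Its construction script adds a spline mesh component per segment, matching neighboring points' local positions and tangents.
; Each segment gets a material picked from an array by the SelectMaterial setting, with configurable grunge color and intensity parameters.
; The event graph holds only disabled placeholder events, so the Blueprint adds no runtime logic.
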(fn `UserConstructionScript`
  (locals (`Material instance` :type "Array of MaterialInstance Object Reference"))
  (bind _spline (`self.Spline`))
  (`|ExecutionSequence`
    (:`then_2`
      ;[1 1 1] Cable Spline
      (for _index (range (+ (- (`SplineComponent.GetNumberOfSplinePoints` _spline) 2) 1))
        (`|ExecutionSequence`
          (:`then_0`
            (bind _returnvalue (`AddComponent|NODE_AddSplineMeshComponent-0` :`bManualAttachment` true))
            (`SceneComponent.K2_AttachToComponent` _returnvalue (`self.Spline`) "None" "KeepRelative" "KeepRelative" "KeepRelative" true)
            (bind (_location _tangent) (`SplineComponent.GetLocationAndTangentAtSplinePoint` _spline _index "Local"))
            (bind (_location_2 _tangent_2) (`SplineComponent.GetLocationAndTangentAtSplinePoint` _spline (+ _index 1) "Local"))
            (`SplineMeshComponent.SetStartAndEnd` _returnvalue _location _tangent _location_2 _tangent_2 true)
            ;[1 1 1] Material
            (`PrimitiveComponent.SetMaterial` _returnvalue 0 (`|GetArrayItem` (`local.Material instance`) (`KismetMathLibrary.Conv_ByteToInt` (`.MaxValue` (`KismetMathLibrary.MaxOfByteArray` (`|MakeArray` (`self.Select Material`) :!type "Byte"))))))
            (`|ExecutionSequence`
              (:`then_0`
                (`MeshComponent.SetVectorParameterValueOnMaterials` _returnvalue "COLOR_GRUNGE" (`KismetMathLibrary.Conv_LinearColorToVector` (`self.Color Grunge`))))
              (:`then_1`
                (`MeshComponent.SetScalarParameterValueOnMaterials` _returnvalue "GRUNGE_ALL" (`self.Grunge Intensity`))))))))))